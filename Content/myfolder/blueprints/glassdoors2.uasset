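; A double sliding door Blueprint, likely glass, that opens once an enemy-related count passes a threshold.
; Each call to the enemycountslidedoors2 custom event increments Enemystuff and compares it against Minstuff.
; Above the threshold, two timelines play to lerp Cube and Cube1 outward in opposite directions along local X.
; The file contains no closing logic, and its construction script is empty.
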(event Custom|enemycountslidedoors2
  (bind _result (Math|Integer|IncrementInt (Variables|Default|Getenemystuff))
    (:%20%20
      (if (> _result (Variables|Default|Getminstuff))
        (Utilities|FlowControl|Sequence
          (:then_0
            (bind _newtrack_0 (Timeline|open%20door%20leftr Play)
              (:Update
                (Transformation|SetRelativeLocation (Variables|Default|GetCube) (Math|Vector|Lerp(Vector) "-250.000000, 0, 0" "-340.000000,0.000000, 0" _newtrack_0) false false))))
          (:then_1
            (bind _newtrack_0_2 (Timeline|Timeline_0 Play)
              (:Update
                (Transformation|SetRelativeLocation (Variables|Default|GetCube1) (Math|Vector|Lerp(Vector) "250.000000, 0, 0" "340.000000,0.000000, 0" _newtrack_0_2) false false)))))))))

(event EventBeginPlay)

(event Collision|EventActorBeginOverlap
  (params (OtherActor :type Actor%20Object%20Reference)))

(event EventTick
  (params (DeltaSeconds :type Float%20%28single-precision%29)))

(event Input|KeyboardEvents|J
  (params (Key :type Key%20Structure :default "None")))

(fn ConstructionScript)