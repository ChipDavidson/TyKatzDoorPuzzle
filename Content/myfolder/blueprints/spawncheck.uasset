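; Trigger actor that spawns a one-time wave of enemy AI when the first-person player character enters its box volume.
; The box overlap casts to FirstPersonCharacter_h, then a DoOnce gate keeps the wave from repeating.
; A Sequence then calls SpawnAIFromClass for Enemy_Character at each of twenty hand-placed location components.
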(event OnComponentBeginOverlap(Box)
  (params (OverlappedComponent :type Primitive%20Component%20Object%20Reference) (OtherActor :type Actor%20Object%20Reference) (OtherComp :type Primitive%20Component%20Object%20Reference) (OtherBodyIndex :type Integer) (bFromSweep :type Boolean) (SweepResult :type Hit%20Result%20Structure%20%28by%20ref%29))
  (Utilities|Casting|CastToFirstPersonCharacter_h OtherActor)
  (Utilities|FlowControl|DoOnce false
    (:Completed
      (Utilities|FlowControl|Sequence
        (:then_0
          (AI|SpawnAIFromClass "/Game/Blueprints/Enemy_Character.Enemy_Character_C" 0 (Transformation|GetWorldLocation (Variables|Default|Getloc1)) "0, 0, 0" false 0))
        (:then_1
          (AI|SpawnAIFromClass "/Game/Blueprints/Enemy_Character.Enemy_Character_C" 0 (Transformation|GetWorldLocation (Variables|Default|Getloc2)) "0, 0, 0" false 0))
        (:then_2
          (AI|SpawnAIFromClass "/Game/Blueprints/Enemy_Character.Enemy_Character_C" 0 (Transformation|GetWorldLocation (Variables|Default|Getloc3)) "0, 0, 0" false 0))
        (:then_3
          (AI|SpawnAIFromClass "/Game/Blueprints/Enemy_Character.Enemy_Character_C" 0 (Transformation|GetWorldLocation (Variables|Default|Getloc4)) "0, 0, 0" false 0))
        (:then_4
          (AI|SpawnAIFromClass "/Game/Blueprints/Enemy_Character.Enemy_Character_C" 0 (Transformation|GetWorldLocation (Variables|Default|Getloc5)) "0, 0, 0" false 0))
        (:then_5
          (AI|SpawnAIFromClass "/Game/Blueprints/Enemy_Character.Enemy_Character_C" 0 (Transformation|GetWorldLocation (Variables|Default|Getloc6)) "0, 0, 0" false 0))
        (:then_6
          (AI|SpawnAIFromClass "/Game/Blueprints/Enemy_Character.Enemy_Character_C" 0 (Transformation|GetWorldLocation (Variables|Default|Getloc7)) "0, 0, 0" false 0))
        (:then_7
          (AI|SpawnAIFromClass "/Game/Blueprints/Enemy_Character.Enemy_Character_C" 0 (Transformation|GetWorldLocation (Variables|Default|Getloc8)) "0, 0, 0" false 0))
        (:then_8
          (AI|SpawnAIFromClass "/Game/Blueprints/Enemy_Character.Enemy_Character_C" 0 (Transformation|GetWorldLocation (Variables|Default|Getloc9)) "0, 0, 0" false 0))
        (:then_9
          (AI|SpawnAIFromClass "/Game/Blueprints/Enemy_Character.Enemy_Character_C" 0 (Transformation|GetWorldLocation (Variables|Default|Getloc10)) "0, 0, 0" false 0))
        (:then_10
          (AI|SpawnAIFromClass "/Game/Blueprints/Enemy_Character.Enemy_Character_C" 0 (Transformation|GetWorldLocation (Variables|Default|Getloc11)) "0, 0, 0" false 0))
        (:then_11
          (AI|SpawnAIFromClass "/Game/Blueprints/Enemy_Character.Enemy_Character_C" 0 (Transformation|GetWorldLocation (Variables|Default|Getloc12)) "0, 0, 0" false 0))
        (:then_12
          (AI|SpawnAIFromClass "/Game/Blueprints/Enemy_Character.Enemy_Character_C" 0 (Transformation|GetWorldLocation (Variables|Default|Getloc13)) "0, 0, 0" false 0))
        (:then_13
          (AI|SpawnAIFromClass "/Game/Blueprints/Enemy_Character.Enemy_Character_C" 0 (Transformation|GetWorldLocation (Variables|Default|Getloc14)) "0, 0, 0" false 0))
        (:then_14
          (AI|SpawnAIFromClass "/Game/Blueprints/Enemy_Character.Enemy_Character_C" 0 (Transformation|GetWorldLocation (Variables|Default|Getloc15)) "0, 0, 0" false 0))
        (:then_15
          (AI|SpawnAIFromClass "/Game/Blueprints/Enemy_Character.Enemy_Character_C" 0 (Transformation|GetWorldLocation (Variables|Default|Getloc16)) "0, 0, 0" false 0))
        (:then_16
          (AI|SpawnAIFromClass "/Game/Blueprints/Enemy_Character.Enemy_Character_C" 0 (Transformation|GetWorldLocation (Variables|Default|Getloc17)) "0, 0, 0" false 0))
        (:then_17
          (AI|SpawnAIFromClass "/Game/Blueprints/Enemy_Character.Enemy_Character_C" 0 (Transformation|GetWorldLocation (Variables|Default|Getloc18)) "0, 0, 0" false 0))
        (:then_18
          (AI|SpawnAIFromClass "/Game/Blueprints/Enemy_Character.Enemy_Character_C" 0 (Transformation|GetWorldLocation (Variables|Default|Getloc19)) "0, 0, 0" false 0))
        (:then_19
          (AI|SpawnAIFromClass "/Game/Blueprints/Enemy_Character.Enemy_Character_C" 0 (Transformation|GetWorldLocation (Variables|Default|Getloc20)) "0, 0, 0" false 0))))))

(event EventBeginPlay)

(event Collision|EventActorBeginOverlap
  (params (OtherActor :type Actor%20Object%20Reference)))

(event EventTick
  (params (DeltaSeconds :type Float%20%28single-precision%29)))

(fn ConstructionScript)