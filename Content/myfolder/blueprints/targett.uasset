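; A shootable target Blueprint that slides along a path and, when hit, triggers a coffin lid to move.
; The construction script builds four relative control points from location variables for an InterpToMovement component, along with a configurable duration.
; A hit on the Hitbox calls Movedalid on the referenced LidActivate object and then hides the Target component.
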(event OnComponentHit(hitbox)
  (params (HitComponent :type Primitive%20Component%20Object%20Reference) (OtherActor :type Actor%20Object%20Reference) (OtherComp :type Primitive%20Component%20Object%20Reference) (NormalImpulse :type Vector :default "0, 0, 0") (Hit :type Hit%20Result%20Structure%20%28by%20ref%29))
  ;[1 1 1] moves lid of coffin
  (Utilities|FlowControl|Sequence
    (:then_0
      (Default|Movedalid (Variables|Default|Getlid_activate)))
    (:then_1
      (Rendering|SetVisibility (Variables|Default|Gettarget) false false))))

(fn ConstructionScript
  (bind _interptomovement (Variables|Default|GetInterpToMovement))
  ;[1 1 1] makes moiving points that ping pong
  (Variables|/Script/Engine.InterpToMovementComponent|SetControlPoints _interptomovement (Utilities|Array|MakeArray (Utilities|Struct|MakeInterpControlPoint (Variables|Default|GetL1) true) (Utilities|Struct|MakeInterpControlPoint (Variables|Default|GetL2) true) (Utilities|Struct|MakeInterpControlPoint (Variables|Default|GetL3) true) (Utilities|Struct|MakeInterpControlPoint (Variables|Default|GetL4) true)))
  (Variables|/Script/Engine.InterpToMovementComponent|SetDuration _interptomovement (Variables|Default|GetDuration)))