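; Falling-platform Blueprint with two cubes that are held in place until their paired box components register a hit.
; BeginPlay disables gravity on Cube2 and Cube3.
; A component hit on Box re-enables gravity for Cube2 and one on Box1 does the same for Cube3, each through its own DoOnce so it fires a single time.
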(event OnComponentHit(Box)
  (params (HitComponent :type Primitive%20Component%20Object%20Reference) (OtherActor :type Actor%20Object%20Reference) (OtherComp :type Primitive%20Component%20Object%20Reference) (NormalImpulse :type Vector :default "0, 0, 0") (Hit :type Hit%20Result%20Structure%20%28by%20ref%29))
  ;[1 1 1] sets gravity
  (Utilities|FlowControl|DoOnce false
    (:Completed
      (Physics|SetEnableGravity (Variables|Default|GetCube2) true))))

(event OnComponentHit(Box1)
  (params (HitComponent :type Primitive%20Component%20Object%20Reference) (OtherActor :type Actor%20Object%20Reference) (OtherComp :type Primitive%20Component%20Object%20Reference) (NormalImpulse :type Vector :default "0, 0, 0") (Hit :type Hit%20Result%20Structure%20%28by%20ref%29))
  ;[1 1 1] sets gravity
  (Utilities|FlowControl|DoOnce false
    (:Completed
      (Physics|SetEnableGravity (Variables|Default|GetCube3) true))))

(event EventBeginPlay
  ;[1 1 1] lock gravity
  (Utilities|FlowControl|Sequence
    (:then_0
      (Physics|SetEnableGravity (Variables|Default|GetCube3) false))
    (:then_1
      (Physics|SetEnableGravity (Variables|Default|GetCube2) false))))

(fn ConstructionScript)