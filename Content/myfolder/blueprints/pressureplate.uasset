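; Pressure plate Blueprint that starts a parkour section and can raise an altar mesh.
; Overlapping the Setparkour trigger with an actor whose display name contains "character" calls a parkour-time event on four referenced objects in sequence.
; A separate raisealter event, not called within this graph, plays the Raise timeline to lerp the Alter component's relative location upward along Z.
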(event OnComponentBeginOverlap(setparkour)
  (params (OverlappedComponent :type Primitive%20Component%20Object%20Reference) (OtherActor :type Actor%20Object%20Reference) (OtherComp :type Primitive%20Component%20Object%20Reference) (OtherBodyIndex :type Integer) (bFromSweep :type Boolean) (SweepResult :type Hit%20Result%20Structure%20%28by%20ref%29))
  ;[1 1 1] trigger box to raise alter for parkour
  (if (Utilities|String|Contains (Utilities|GetDisplayName OtherActor) "character")
    (Utilities|FlowControl|Sequence
      (:then_0
        (Default|Parkourtime1 (Variables|Default|Getraiseup)))
      (:then_1
        (Default|Parkourtime2 (Variables|Default|Getparkour2)))
      (:then_2
        (Default|Parkourtime3 (Variables|Default|Getparkour3)))
      (:then_3
        (Default|Parkourtime4 (Variables|Default|Getparkour4))))))

(event Custom|raisealter
  ;[1 1 1] raises alter with event
  (bind _newtrack_0 (Timeline|raise Play)
    (:Update
      (Transformation|SetRelativeLocation (Variables|Default|Getalter) (Math|Vector|Lerp(Vector) "0, 0, 0" "0, 0,130.000000" _newtrack_0) false false))))

(fn ConstructionScript)