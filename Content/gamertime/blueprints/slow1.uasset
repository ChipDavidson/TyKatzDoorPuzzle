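; Slow-down hazard Blueprint that temporarily reduces the first player's walk speed when its Box component is hit.
; On hit it sets the character's max walk speed to 200, restores 600 after a four-second delay, and hides the Tarjet component.
; The hit handler does not check which actor hit it, and the actor is never destroyed.
; Disconnected leftover nodes for disabling movement, stopping movement and changing FOV never run.
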(event OnComponentHit(Box)
  (params (HitComponent :type Primitive%20Component%20Object%20Reference) (OtherActor :type Actor%20Object%20Reference) (OtherComp :type Primitive%20Component%20Object%20Reference) (NormalImpulse :type Vector :default "0, 0, 0") (Hit :type Hit%20Result%20Structure%20%28by%20ref%29))
  (bind _returnvalue (Game|GetPlayerCharacter 0))
  (bind _charactermovement (Variables|/Script/Engine.Character|GetCharacterMovement _returnvalue))
  ;[1 1 1] slow player
  (Utilities|FlowControl|Sequence
    (:then_0
      (Variables|/Script/Engine.CharacterMovementComponent|SetMaxWalkSpeed _charactermovement 2e+02)
      (Utilities|FlowControl|Delay 4.0)
      (Variables|/Script/Engine.CharacterMovementComponent|SetMaxWalkSpeed _charactermovement 6e+02))
    (:then_1
      (Rendering|SetVisibility (Variables|Default|Gettarjet) false false))))

(fn ConstructionScript)