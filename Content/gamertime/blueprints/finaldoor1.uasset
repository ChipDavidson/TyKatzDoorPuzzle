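; Final door actor: a cell door that swings open when its box component is hit.
; The hit plays a timeline that drives the door mesh's relative yaw, with no filter on what hit it, as the "character" name check is disconnected.
; A separate showskull event makes the Tarjet component visible.
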(event OnComponentHit(Box)
  (params (HitComponent :type Primitive%20Component%20Object%20Reference) (OtherActor :type Actor%20Object%20Reference) (OtherComp :type Primitive%20Component%20Object%20Reference) (NormalImpulse :type Vector :default "0, 0, 0") (Hit :type Hit%20Result%20Structure%20%28by%20ref%29))
  (Utilities|FlowControl|Sequence
    (:then_0
      (bind _dooropen (Timeline|Timeline_1 Play)
        (:Update
          (Transformation|SetRelativeRotation (Variables|Default|GetSM_Cell_Door) (Math|Rotator|MakeRotator 0.0 0.0 _dooropen) false false))))))

(event Custom|showskull
  (Rendering|SetVisibility (Variables|Default|Gettarjet) true false))

(fn ConstructionScript)