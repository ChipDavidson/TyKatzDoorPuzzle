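; Door Blueprint for a pair of large crypt doors that swing open.
; The opensesame event plays two timelines, each driving one leaf's yaw through relative rotation.
; A box overlap does the same with its own pair of timelines when the overlapping actor's display name contains "character", a string match rather than a cast.
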(event OnComponentBeginOverlap(Box)
  (params (OverlappedComponent :type Primitive%20Component%20Object%20Reference) (OtherActor :type Actor%20Object%20Reference) (OtherComp :type Primitive%20Component%20Object%20Reference) (OtherBodyIndex :type Integer) (bFromSweep :type Boolean) (SweepResult :type Hit%20Result%20Structure%20%28by%20ref%29))
  (if (Utilities|String|Contains (Utilities|GetDisplayName OtherActor) "character")
    (Utilities|FlowControl|Sequence
      (:then_0
        (bind _dooropen (Timeline|Timeline_2 Play)
          (:Update
            (Transformation|SetRelativeRotation (Variables|Default|GetSM_DoorWay_Large_Door_Right) (Math|Rotator|MakeRotator 0.0 0.0 _dooropen) false false))))
      (:then_1
        (bind _dooropen_2 (Timeline|Timeline_3 Play)
          (:Update
            (Transformation|SetRelativeRotation (Variables|Default|GetSM_DoorWay_Large_Door_Left) (Math|Rotator|MakeRotator 0.0 0.0 _dooropen_2) false false)))))))

(event Custom|opensesame
  ;[1 1 1] event to open crypt doors
  (Utilities|FlowControl|Sequence
    (:then_0
      (bind _dooropen (Timeline|Timeline_1 Play)
        (:Update
          (Transformation|SetRelativeRotation (Variables|Default|GetSM_DoorWay_Large_Door_Right) (Math|Rotator|MakeRotator 0.0 0.0 _dooropen) false false))))
    (:then_1
      (bind _dooropen_2 (Timeline|Timeline_0 Play)
        (:Update
          (Transformation|SetRelativeRotation (Variables|Default|GetSM_DoorWay_Large_Door_Left) (Math|Rotator|MakeRotator 0.0 0.0 _dooropen_2) false false))))))

(fn ConstructionScript)