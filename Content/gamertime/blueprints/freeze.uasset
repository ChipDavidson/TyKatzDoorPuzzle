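; Freeze trap actor that stun-locks the player when its Box component registers a hit.
; The first hit shows a Stun widget and disables player 0's movement for two seconds, then restores walking and removes the widget.
; Every hit hides the Tarjet component, while a DoOnce keeps the stun single-use.
; Disconnected nodes hold unused movement-stop, slow and FOV experiments.
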(event OnComponentHit(Box)
  (params (HitComponent :type Primitive%20Component%20Object%20Reference) (OtherActor :type Actor%20Object%20Reference) (OtherComp :type Primitive%20Component%20Object%20Reference) (NormalImpulse :type Vector :default "0, 0, 0") (Hit :type Hit%20Result%20Structure%20%28by%20ref%29))
  ;[1 1 1] stun lock cc
  (Utilities|FlowControl|Sequence
    (:then_0
      (Utilities|FlowControl|DoOnce false
        (:Completed
          (bind _returnvalue (UserInterface|CreateWidget "/Game/gamertime/blueprints/stun.stun_C"))
          (UserInterface|Viewport|AddtoViewport _returnvalue 0)
          (Pawn|Components|CharacterMovement|DisableMovement (Variables|/Script/Engine.Character|GetCharacterMovement (Game|GetPlayerCharacter 0)))
          (Utilities|FlowControl|Delay 2.0)
          (Pawn|Components|CharacterMovement|SetMovementMode (Variables|/Script/Engine.Character|GetCharacterMovement (Game|GetPlayerCharacter 0)) "MOVE_Walking" 0)
          (Widget|RemovefromParent _returnvalue))))
    (:then_1
      (Rendering|SetVisibility (Variables|Default|Gettarjet) false false))))

(fn ConstructionScript)